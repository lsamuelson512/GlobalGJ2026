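; Game instance for ColorMask that owns the save data and persists the player's MaxL and MaxR values.
; On Init it loads the "Save" slot into SaveRef, or creates and writes a new SG_Save if none exists.
; SaveGame writes both values to that slot, LoadGame copies them from SaveRef onto a given player, and DeleteGame deletes the slot.
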(event `self.ReceiveInit`
  (bind _returnvalue (`GameplayStatics.DoesSaveGameExist` "Save"))
  (if _returnvalue
    (bind _returnvalue_2 (`GameplayStatics.LoadGameFromSlot` "Save"))
    (bind _assg_save (cast `/Game/Blueprints/Core/SG_Save` _returnvalue_2))
    (set `self.SaveRef` _assg_save)
    (else
      (bind _returnvalue_3 (`GameplayStatics.CreateSaveGameObject` "/Game/Blueprints/Core/SG_Save.SG_Save_C"))
      (bind _output_get (set `self.SaveRef` _returnvalue_3))
      (`GameplayStatics.SaveGameToSlot` _output_get "Save"))))

(event `/Game/Blueprints/Core/BPI_SaveAndLoad.SaveGame`
  (params (MaxL :type "Float (double-precision)") (MaxR :type "Float (double-precision)"))
  (bind _saveref (`self.SaveRef`))
  (set `/Game/Blueprints/Core/SG_Save.MaxL` MaxL _saveref)
  (set `/Game/Blueprints/Core/SG_Save.MaxR` MaxR _saveref)
  (`GameplayStatics.SaveGameToSlot` _saveref "Save"))

(event `/Game/Blueprints/Core/BPI_SaveAndLoad.DeleteGame`
  (`GameplayStatics.DeleteGameInSlot` "Save"))

(fn `LoadGame`
  (params (PlayerRef :type "/Game/Blueprints/Core/BP_FirstPersonCharacter Object Reference"))
  (bind _saveref (`self.SaveRef`))
  (set `/Game/Blueprints/Core/BP_FirstPersonCharacter.MaxL` (`/Game/Blueprints/Core/SG_Save.MaxL` _saveref) PlayerRef)
  (set `/Game/Blueprints/Core/BP_FirstPersonCharacter.MaxR` (`/Game/Blueprints/Core/SG_Save.MaxR` _saveref) PlayerRef)
  (return))