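; BP_HoleInWall is a spawner that sends out BP_Walls actors at its own transform until the player reaches an objective.
; Spawning starts on BeginPlay, and the SpawnWalls event re-calls itself after a three-second delay to form a repeating loop.
; When the player character overlaps its Box component, a ReachedObj flag is set, which ends the loop after the pending delay.
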(event `self.ReceiveBeginPlay`
  (`self.SpawnWalls`))

(event `SpawnWalls`
  (`|SpawnActorFromClass` "/Game/Blueprints/BP_Walls.BP_Walls_C" (`self.GetTransform`) "Undefined" "MultiplyWithRoot" self null)
  (`KismetSystemLibrary.Delay` 3.0)
  (if (not (`self.ReachedObj`))
    (`self.SpawnWalls`)))

(event `self.Box.OnComponentBeginOverlap`
  (params (OverlappedComponent :type "PrimitiveComponent Object Reference") (OtherActor :type "Actor Object Reference") (OtherComp :type "PrimitiveComponent Object Reference") (OtherBodyIndex :type Integer) (bFromSweep :type Boolean) (SweepResult :type "HitResult Structure (by ref)"))
  (if (== OtherActor (`GameplayStatics.GetPlayerCharacter` 0))
    (set `self.ReachedObj` true)))

(fn `UserConstructionScript`)