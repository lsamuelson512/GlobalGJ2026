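; BP_NumPad is a keypad-locked double door that the player opens through a numpad widget.
; BeginPlay creates W_NumPad and passes it the solution, color formatting and a self reference.
; The Box overlap shows or hides the widget for the player, switching input mode and cursor, unless Opened is set.
; OpenDoor removes the widget, then slides both doors apart with a per-frame zero-Delay Lerp loop.
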(event `self.ReceiveBeginPlay`
  (bind _returnvalue (`|CreateWidget` "/Game/Widgets/W_NumPad.W_NumPad_C"))
  (bind _output_get (set `self.WPadRef` _returnvalue))
  (set `/Game/Widgets/W_NumPad.ColorFormating` (`self.ColorFormatting`) _output_get)
  (set `/Game/Widgets/W_NumPad.Solution` (`self.Solution`) _output_get)
  (set `/Game/Widgets/W_NumPad.NumPadRef` self _output_get))

(event `self.Box.OnComponentBeginOverlap`
  (params (OverlappedComponent :type "PrimitiveComponent Object Reference") (OtherActor :type "Actor Object Reference") (OtherComp :type "PrimitiveComponent Object Reference") (OtherBodyIndex :type Integer) (bFromSweep :type Boolean) (SweepResult :type "HitResult Structure (by ref)"))
  (bind _returnvalue (`GameplayStatics.GetPlayerController` 0))
  (bind _wpadref (`self.WPadRef`))
  (if (and (== OtherActor (`GameplayStatics.GetPlayerCharacter` 0)) (not (`self.Opened?`)))
    (`UserWidget.AddToViewport` _wpadref 0)
    (`WidgetBlueprintLibrary.SetInputMode_UIOnlyEx` _returnvalue (`/Game/Widgets/W_NumPad.>` _wpadref) "DoNotLock" true)
    (set `PlayerController.bShowMouseCursor` true _returnvalue)))

(event `self.Box.OnComponentEndOverlap`
  (params (OverlappedComponent :type "PrimitiveComponent Object Reference") (OtherActor :type "Actor Object Reference") (OtherComp :type "PrimitiveComponent Object Reference") (OtherBodyIndex :type Integer))
  (bind _returnvalue (`GameplayStatics.GetPlayerController` 0))
  (if (and (== OtherActor (`GameplayStatics.GetPlayerCharacter` 0)) (not (`self.Opened?`)))
    (`WidgetBlueprintLibrary.SetInputMode_GameOnly` _returnvalue)
    (set `PlayerController.bShowMouseCursor` false _returnvalue)
    (`Widget.RemoveFromParent` (`self.WPadRef`))))

(event `OpenDoor`
  (`Widget.RemoveFromParent` (`self.WPadRef`))
  (bind _output_get (set `self.DeltaTime` (+ (`self.DeltaTime`) (`GameplayStatics.GetWorldDeltaSeconds`)) :!label _label))
  (bind _returnvalue (`KismetMathLibrary.Lerp` 111.0 250.0 (/ _output_get (`self.Duration`))))
  (`SceneComponent.K2_SetRelativeLocation` (`self.DoorR`) (`KismetMathLibrary.MakeVector` _returnvalue 0.0 -250.0) false false)
  (`SceneComponent.K2_SetRelativeLocation` (`self.DoorL`) (`KismetMathLibrary.MakeVector` (* _returnvalue -1.0) 0.0 -250.0) false false)
  (if (< (`self.DeltaTime`) (`self.Duration`))
    (`KismetSystemLibrary.Delay` 0.0)
    (goto _label)))

(fn `UserConstructionScript`)