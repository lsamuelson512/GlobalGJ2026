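; BP_Hammer is a swinging pendulum hammer obstacle that knocks the player character away on contact.
; A self-calling event with a zero Delay eases SwingPoint's pitch sinusoidally between plus and minus HalfAngle, flipping direction at either end of Duration.
; Right and Left overlaps launch the player in opposite directions relative to SwingPoint's rotation, with fixed upward velocity.
; BeginPlay also sets both cylinders' custom depth stencil value.
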(event `self.ReceiveBeginPlay`
  (`PrimitiveComponent.SetCustomDepthStencilValue` (`self.Cylinder`) (`self.Depth`))
  (`PrimitiveComponent.SetCustomDepthStencilValue` (`self.Cylinder1`) (`self.Depth`))
  (`self.SwingingPendulum`))

(event `SwingingPendulum`
  (bind _halfangle (`self.HalfAngle`))
  (bind _delttime (`self.DeltTime`))
  (bind _output_get (set `self.DeltTime` (+ (* (`GameplayStatics.GetWorldDeltaSeconds`) (`self.Direction`)) (`self.DeltTime`))))
  (`SceneComponent.K2_SetRelativeRotation` (`self.SwingPoint`) (`KismetMathLibrary.MakeRotator` 0.0 (`|EaseFunction` "SinusoidalInOut" (/ _output_get (`self.Duration`)) (* _halfangle -1.0) _halfangle)) false false)
  (if (or (< _delttime 0.01) (> _delttime (`self.Duration`)))
    (set `self.Direction` (* (`self.Direction`) -1.0)))
  (`KismetSystemLibrary.Delay` 0.0)
  (`self.SwingingPendulum`))

(event `self.Right.OnComponentBeginOverlap`
  (params (OverlappedComponent :type "PrimitiveComponent Object Reference") (OtherActor :type "Actor Object Reference") (OtherComp :type "PrimitiveComponent Object Reference") (OtherBodyIndex :type Integer) (bFromSweep :type Boolean) (SweepResult :type "HitResult Structure (by ref)"))
  (bind _returnvalue (`GameplayStatics.GetPlayerCharacter` 0))
  (bind (_returnvalue_roll _returnvalue_pitch _returnvalue_yaw) (`KismetMathLibrary.BreakRotator` (`SceneComponent.K2_GetComponentRotation` (`self.SwingPoint`))))
  (bind (_returnvalue_x _returnvalue_y) (`KismetMathLibrary.BreakVector` (`KismetMathLibrary.GreaterGreater_VectorRotator` (1500.0 1500.0 0.0) (`KismetMathLibrary.MakeRotator` _returnvalue_roll _returnvalue_pitch (+ _returnvalue_yaw -45.0)))))
  (if (== OtherActor _returnvalue)
    (`Character.LaunchCharacter` _returnvalue (`KismetMathLibrary.MakeVector` _returnvalue_x _returnvalue_y 500.0) true false)))

(event `self.Left.OnComponentBeginOverlap`
  (params (OverlappedComponent :type "PrimitiveComponent Object Reference") (OtherActor :type "Actor Object Reference") (OtherComp :type "PrimitiveComponent Object Reference") (OtherBodyIndex :type Integer) (bFromSweep :type Boolean) (SweepResult :type "HitResult Structure (by ref)"))
  (bind _returnvalue (`GameplayStatics.GetPlayerCharacter` 0))
  (bind (_returnvalue_roll _returnvalue_pitch _returnvalue_yaw) (`KismetMathLibrary.BreakRotator` (`SceneComponent.K2_GetComponentRotation` (`self.SwingPoint`))))
  (bind (_returnvalue_x _returnvalue_y) (`KismetMathLibrary.BreakVector` (`KismetMathLibrary.GreaterGreater_VectorRotator` (1500.0 1500.0 0.0) (`KismetMathLibrary.MakeRotator` _returnvalue_roll _returnvalue_pitch (+ _returnvalue_yaw 135.0)))))
  (if (== OtherActor _returnvalue)
    (`Character.LaunchCharacter` _returnvalue (`KismetMathLibrary.MakeVector` _returnvalue_x _returnvalue_y 500.0) true false)))

(fn `UserConstructionScript`)