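; BP_MovingBumper is a moving obstacle that knocks the player character away on contact.
; A self-repeating zero-Delay loop moves its mesh along a spline at constant velocity, reversing direction at each end of the duration.
; Capsule overlap launches the player with a fixed vector rotated by the bumper-to-player look-at rotation, plus upward lift.
; BeginPlay also sets the mesh's custom depth stencil value.
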(event `self.ReceiveBeginPlay`
  (`PrimitiveComponent.SetCustomDepthStencilValue` (`self.StaticMesh`) (`self.Depth`))
  (`self.MoveBumper`))

(event `MoveBumper`
  (bind _delttime (`self.DeltTime`))
  (bind _output_get (set `self.DeltTime` (+ (* (`GameplayStatics.GetWorldDeltaSeconds`) (`self.Direction`)) (`self.DeltTime`))))
  (`SceneComponent.K2_SetRelativeLocation` (`self.StaticMesh`) (`SplineComponent.GetLocationAtTime` (`self.Spline`) (/ _output_get (`self.Duration`)) "Local" true) false false)
  (if (or (< _delttime 0.01) (> _delttime (`self.Duration`)))
    (set `self.Direction` (* (`self.Direction`) -1.0)))
  (`KismetSystemLibrary.Delay` 0.0)
  (`self.MoveBumper`))

(event `self.Capsule.OnComponentBeginOverlap`
  (params (OverlappedComponent :type "PrimitiveComponent Object Reference") (OtherActor :type "Actor Object Reference") (OtherComp :type "PrimitiveComponent Object Reference") (OtherBodyIndex :type Integer) (bFromSweep :type Boolean) (SweepResult :type "HitResult Structure (by ref)"))
  (bind _returnvalue (`GameplayStatics.GetPlayerCharacter` 0))
  (bind (_returnvalue_x _returnvalue_y) (`KismetMathLibrary.BreakVector` (`KismetMathLibrary.GreaterGreater_VectorRotator` (2000.0 2000.0 0.0) (`KismetMathLibrary.FindLookAtRotation` (`SceneComponent.K2_GetComponentLocation` (`self.StaticMesh`)) (`self.K2_GetActorLocation` _returnvalue)))))
  (if (== OtherActor _returnvalue)
    (`Character.LaunchCharacter` _returnvalue (`KismetMathLibrary.MakeVector` _returnvalue_x _returnvalue_y 250.0) true false)))

(fn `UserConstructionScript`)