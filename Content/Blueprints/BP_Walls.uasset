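; Moving wall obstacle actor that spawns two wall pieces with random complementary lengths, slides them along X, then destroys itself.
; BeginPlay splits a fixed total scale between LeftWall and RightWall using a randomly seeded integer, then starts movement after a short delay.
; MoveWalls re-calls itself through a zero Delay as a per-frame loop, lerping both walls from the owner's X to EndX over Duration.
; RandomizeWallLengths is an empty stub.
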(event `self.ReceiveBeginPlay`
  (bind _output_get (set `self.RandInterior` (`KismetMathLibrary.RandomIntegerFromStream` (`KismetMathLibrary.MakeRandomStream` (`KismetMathLibrary.RandomInteger` 999)) 6)))
  (`SceneComponent.SetWorldScale3D` (`self.LeftWall`) (`KismetMathLibrary.MakeVector` (`KismetMathLibrary.Conv_IntToDouble` _output_get) 1.0 2.0))
  (`SceneComponent.SetWorldScale3D` (`self.RightWall`) (`KismetMathLibrary.MakeVector` 1.0 (`KismetMathLibrary.Conv_IntToDouble` (- 8 (+ _output_get 2))) 2.0))
  (`KismetSystemLibrary.Delay` 0.2)
  (`self.MoveWalls`))

(event `MoveWalls`
  (bind _leftwall (`self.LeftWall`))
  (bind _rightwall (`self.RightWall`))
  (bind (_returnvalue_x _returnvalue_y _returnvalue_z) (`KismetMathLibrary.BreakVector` (`SceneComponent.K2_GetComponentLocation` _leftwall)))
  (bind _returnvalue_x_2 (`KismetMathLibrary.BreakVector` (`self.K2_GetActorLocation` (`self.GetOwner`))))
  (bind (_returnvalue_x_3 _returnvalue_y_2 _returnvalue_z_2) (`KismetMathLibrary.BreakVector` (`SceneComponent.K2_GetComponentLocation` _rightwall)))
  (bind _returnvalue (`KismetMathLibrary.Lerp` _returnvalue_x_2 (`self.EndX`) (`KismetMathLibrary.FClamp` (/ (`self.Delta`) (`self.Duration`)))))
  (set `self.Delta` (+ (`self.Delta`) (`GameplayStatics.GetWorldDeltaSeconds`)))
  (`SceneComponent.K2_SetWorldLocation` _leftwall (`KismetMathLibrary.MakeVector` _returnvalue _returnvalue_y _returnvalue_z) false false)
  (`SceneComponent.K2_SetWorldLocation` _rightwall (`KismetMathLibrary.MakeVector` _returnvalue _returnvalue_y_2 _returnvalue_z_2) false false)
  (if (> (`self.Delta`) (`self.Duration`))
    (`KismetSystemLibrary.Delay` 1.0)
    (`self.K2_DestroyActor`)
    (else
      (`KismetSystemLibrary.Delay` 0.0)
      (`self.MoveWalls`))))

(fn `RandomizeWallLengths`
  (returns (Left :type Integer) (Right :type Integer))
  (locals (RandInt :type Integer :default 0)))

(fn `UserConstructionScript`)